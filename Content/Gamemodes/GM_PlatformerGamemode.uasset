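; Platformer game mode that owns score, player death, music and the player's HUD.
; On BeginPlay it sets the master sound mix, starts HarmonyCue and adds the player stats and pickup prompt widgets.
; Death and score events play cues through SpawnSFX, which pauses the music until the effect finishes; death also destroys the character.
; Score clamps at ScoreLimit and fires WinGame, which is empty here.
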(event Custom|Event%20PlayerDied
  (CallFunction|EventSpawnSFX "/Game/Audio/SoundEffects/PlayerDeath_Cue.PlayerDeath_Cue")
  (Actor|DestroyActor (Game|GetPlayerCharacter 0))
  (Variables|Default|SetPlayerDead true))

(event Custom|Event%20IncreaseScore
  (params (Increment :type Integer))
  (bind _scorelimit (Variables|Default|GetScoreLimit))
  (CallFunction|EventSpawnSFX "/Game/Audio/SoundEffects/GotPoint_Cue.GotPoint_Cue")
  (if (>= (+ Increment (Variables|Default|GetScore)) _scorelimit)
    (Variables|Default|SetScore _scorelimit)
    (CallFunction|EventWinGame)
    (else
      (Variables|Default|SetScore (+ Increment (Variables|Default|GetScore))))))

(event Custom|Event%20WinGame)

(event Custom|Event%20SpawnSFX
  (params (SoundEffect :type Sound%20Base%20Object%20Reference))
  (Class|AudioComponent|SetPaused (Variables|Default|Getharmony_Cue) true)
  (bind _returnvalue (Audio|SpawnSound2D SoundEffect 1.0 1.0 0.0 0))
  (EventDispatchers|BindEventtoOnAudioFinished _returnvalue (delegate Custom|Event%20SFXFinished)))

(event Custom|Event%20SFXFinished
  (Class|AudioComponent|SetPaused (Variables|Default|Getharmony_Cue) false))

(event EventBeginPlay
  (bind _returnvalue (Game|GetPlayerController 0))
  (Class|GameplayStatics|SetBaseSoundMix "/Game/Audio/Mixes/SM_MasterMixer.SM_MasterMixer")
  (Audio|Components|Audio|Play (Variables|Default|Getharmony_Cue) 0.0)
  (bind _returnvalue_2 (UserInterface|CreateWidget "/Game/UI/WB_PlayerStats.WB_PlayerStats_C" _returnvalue))
  (UserInterface|Viewport|AddtoPlayerScreen _returnvalue_2)
  (bind _returnvalue_3 (UserInterface|CreateWidget "/Game/UI/WB_PickupPrompt.WB_PickupPrompt_C" _returnvalue))
  (UserInterface|Viewport|AddtoPlayerScreen _returnvalue_3))

(fn ConstructionScript)